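; Base weapon pickup actor that lets the player swap the held gun for the one on the ground, keeping ammo and identity.
; Gives itself a random gun ID on BeginPlay and shows or hides a pickup HUD prompt on overlap.
; PickupItem spawns a pickup of the held gun, overwrites the matching primary or secondary slot by ID, swaps the Gun child actor class, restores its state, then destroys itself.
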(event Custom|PickupItem
  (bind _pickerupper (Variables|Default|GetPickerUpper))
  ;[1 1 1] Create a new weapon containing the data of the weapon the character was holding, then spawn the dropped weapon
  (bind _asgun_parent (Utilities|Casting|CastToGun_Parent (Variables|/Script/Engine.ChildActorComponent|GetChildActor (Variables|/Game/FirstPerson/Blueprints/BP_FirstPersonCharacter.BP_FirstPersonCharacter_C|GetGun (Variables|Default|GetPickerUpper)))))
  (bind _returnvalue (Game|SpawnActorfromClass (Variables|/Game/Guns/Gun_Parent.Gun_Parent_C|GetPickupClass _asgun_parent) (Transformation|GetActorTransform) "Undefined" 0 0))
  (Variables|BP_Pickup_Gun_Parent_C|SetWeaponState _returnvalue (Utilities|Struct|MakeGunVariables (Utilities|GetClass _asgun_parent) (.ammocurrent (Variables|/Game/Guns/Gun_Parent.Gun_Parent_C|GetAmmoState _asgun_parent)) (.ammomax (Variables|/Game/Guns/Gun_Parent.Gun_Parent_C|GetAmmoState _asgun_parent)) (Variables|/Game/Guns/Gun_Parent.Gun_Parent_C|GetGunName _asgun_parent) (Variables|/Game/Guns/Gun_Parent.Gun_Parent_C|GetUUID _asgun_parent)))
  ;[1 1 1] Replace primary or secondary weapon data with new weapon data
  (if (== (Variables|/Game/Guns/Gun_Parent.Gun_Parent_C|GetUUID _asgun_parent) (.gunid (Variables|/Game/FirstPerson/Blueprints/BP_FirstPersonCharacter.BP_FirstPersonCharacter_C|GetMainWeapon (Variables|Default|GetPickerUpper))))
    (Variables|/Game/FirstPerson/Blueprints/BP_FirstPersonCharacter.BP_FirstPersonCharacter_C|SetMainWeapon _pickerupper (Utilities|Struct|MakeGunVariables (.guntype (Variables|Default|GetWeaponState)) (.ammocurrent (Variables|Default|GetWeaponState)) (.ammomax (Variables|Default|GetWeaponState)) (.name (Variables|Default|GetWeaponState)) (.gunid (Variables|Default|GetWeaponState))))
    (else
      (Variables|/Game/FirstPerson/Blueprints/BP_FirstPersonCharacter.BP_FirstPersonCharacter_C|SetSecondaryWeapon (Variables|Default|GetPickerUpper) (Utilities|Struct|MakeGunVariables (.guntype (Variables|Default|GetWeaponState)) (.ammocurrent (Variables|Default|GetWeaponState)) (.ammomax (Variables|Default|GetWeaponState)) (.name (Variables|Default|GetWeaponState)) (.gunid (Variables|Default|GetWeaponState))))))
  ;;[1 1 1] Change the weapon being held to the new weapon
  (ChildActorComponent|SetChildActorClass (Variables|/Game/FirstPerson/Blueprints/BP_FirstPersonCharacter.BP_FirstPersonCharacter_C|GetGun _pickerupper) (.guntype (Variables|Default|GetWeaponState)))
  ;[1 1 1] Update weapon state
  (bind _asgun_parent_2 (Utilities|Casting|CastToGun_Parent (Variables|/Script/Engine.ChildActorComponent|GetChildActor (Variables|/Game/FirstPerson/Blueprints/BP_FirstPersonCharacter.BP_FirstPersonCharacter_C|GetGun (Variables|Default|GetPickerUpper)))))
  (Utilities|Struct|SetmembersinAmmoState (Variables|/Game/Guns/Gun_Parent.Gun_Parent_C|GetAmmoState _asgun_parent_2) (.ammocurrent (Variables|Default|GetWeaponState)) (.ammomax (Variables|Default|GetWeaponState)))
  (Variables|/Game/Guns/Gun_Parent.Gun_Parent_C|SetUUID _asgun_parent_2 (.gunid (Variables|Default|GetWeaponState)))
  (Variables|/Game/Guns/Gun_Parent.Gun_Parent_C|SetGunName _asgun_parent_2 (.name (Variables|Default|GetWeaponState)))
  ;[1 1 1] Destroy the old weapon on ground
  (Actor|DestroyActor))

(event Collision|EventActorEndOverlap
  (params (OtherActor :type Actor%20Object%20Reference))
  (Variables|Default|SetIsOverlap false)
  ;[1 1 1] Hide pickup HUD when no longer overlapping
  (bind _asfp_controller (Utilities|Casting|CastToFP_Controller (Game|GetPlayerController 0)))
  (Utilities|IsValid (Variables|/Game/UI/FP_Controller.FP_Controller_C|GetHUD _asfp_controller)
    (:Is%20Valid
      (Default|HidePickupWeapon (Variables|/Game/UI/FP_Controller.FP_Controller_C|GetHUD _asfp_controller)))))

(event Collision|EventActorBeginOverlap
  (params (OtherActor :type Actor%20Object%20Reference))
  (Variables|Default|SetIsOverlap true)
  ;[1 1 1] Show pickup HUD when overlapping
  (bind _asfp_controller (Utilities|Casting|CastToFP_Controller (Game|GetPlayerController 0)))
  (Utilities|IsValid (Variables|/Game/UI/FP_Controller.FP_Controller_C|GetHUD _asfp_controller)
    (:Is%20Valid
      (Default|ShowPickupWeapon (Variables|/Game/UI/FP_Controller.FP_Controller_C|GetHUD _asfp_controller) (.name (Variables|Default|GetWeaponState))))))

(event EventBeginPlay
  (Variables|Default|SetWeaponState (Utilities|Struct|MakeGunVariables (.guntype (Variables|Default|GetWeaponState)) (.ammocurrent (Variables|Default|GetWeaponState)) (.ammomax (Variables|Default|GetWeaponState)) (.name (Variables|Default|GetWeaponState)) (Math|Random|RandomIntegerinRange 0 10000))))

(fn ConstructionScript)